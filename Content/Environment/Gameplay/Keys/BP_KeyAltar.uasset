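; BP_KeyAltar is an altar that spends one of the player's keys to fire an activation event.
; When BP_T800_Dora overlaps with a key, it calls OnActivated, reveals the hidden Bonsho bell, rings it and spawns two delayed energy waves.
; Without a key, it plays audio with a subtitle widget that is removed when the audio finishes.
; Interface events expose delegate binding, though IsActivated is never set here and GetState always returns false.
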(event `self.ReceiveBeginPlay`
  (`SceneComponent.SetHiddenInGame` (`self.BonshoBell`) true false))

(event `self.ReceiveActorBeginOverlap`
  (params (OtherActor :type "Actor Object Reference"))
  (if (not (`self.IsActivated`))
    (bind _asbp_t800_dora (cast `/Game/Gameplay/Player/BP_T800_Dora` OtherActor))
    (bind _keycount (`/Game/Gameplay/Player/BP_T800_Dora.KeyCount` _asbp_t800_dora))
    (if (> _keycount 0)
      (`/Engine/EditorBlueprintResources/StandardMacros.DecrementInt` _keycount
        (:`  `
          (`self.OnActivated`)
          (`SceneComponent.SetHiddenInGame` (`self.BonshoBell`) false false)
          (`GameplayStatics.PlaySoundAtLocation` "/Game/Audio/Cue/SC_BonshoRing.SC_BonshoRing" (`self.K2_GetActorLocation`) (struct) 1.0 1.0 0.0 null null null null)
          (`NiagaraFunctionLibrary.SpawnSystemAtLocation` "/Game/Environment/Gameplay/Shockwave/NS_EnergyWave.NS_EnergyWave" (`self.K2_GetActorLocation`) (struct) (5.0 5.0 5.0))
          (`KismetSystemLibrary.Delay` 1.0)
          (`NiagaraFunctionLibrary.SpawnSystemAtLocation` "/Game/Environment/Gameplay/Shockwave/NS_EnergyWave.NS_EnergyWave" (`self.K2_GetActorLocation`) (struct) (5.0 5.0 5.0))))
      (else
        (bind _returnvalue (`|CreateWidget` "/Game/UI/Pages/WBP_SubtitleNoBell.WBP_SubtitleNoBell_C" (`GameplayStatics.GetPlayerController` 0)))
        (bind _output_get (set `self.Widget` _returnvalue))
        (`UserWidget.AddToViewport` _output_get 0)
        (`AudioComponent.Play` (`self.Audio`) 0.0)))))

(event `self.BindEventToOnActivated`
  (params (Delegate :type "Delegate (by ref)"))
  ; Interface links
  (add `self.OnActivated` Delegate))

(event `self.BindEventToOnDeactivated`
  (params (Delegate :type "Delegate (by ref)"))
  ; Interface links
  (add `self.OnDeactivated` Delegate))

(event `self.UnbindEventFromOnActivated`
  (params (Delegate :type "Delegate (by ref)"))
  ; Interface links
  (remove `self.OnActivated` Delegate))

(event `self.Audio.OnAudioFinished`
  (`Widget.RemoveFromParent` (`self.Widget`)))

(event `self.UnbindEventFromOnDeactivated`
  (params (Delegate :type "Delegate (by ref)"))
  ; Interface links
  (remove `self.OnDeactivated` Delegate))

(fn `GetState`
  (returns (ReturnValue :type Boolean))
  (return false))

(fn `UserConstructionScript`)