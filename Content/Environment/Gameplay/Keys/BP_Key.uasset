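; BP_Key is a collectible key that raises BP_T800_Dora's key count on overlap, plays a sound and destroys itself.
; With SpawnOnRoomOver set, it waits a tick, binds to the OnRoomOver event of each BP_RoomBase overlapping its Sphere, then hides through BPCSpawnOnSolve.
; When a bound room signals it is over, the same component shows the key again.
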(event `self.ReceiveBeginPlay`
  (if (`self.SpawnOnRoomOver`)
    (`KismetSystemLibrary.DelayUntilNextTick`)
    (for _array_element (`PrimitiveComponent.GetOverlappingActors` (`self.Sphere`) "/Game/Gameplay/Rooms/BP_RoomBase.BP_RoomBase_C")
      (bind _asbp_room_base (cast `/Game/Gameplay/Rooms/BP_RoomBase` _array_element))
      (add `/Game/Gameplay/Rooms/BP_RoomBase.OnRoomOver` _asbp_room_base (delegate `ShowBack`)))
    (`/Game/Environment/Gameplay/Collectibles/BPC_SpawnOnSolve.Hide` (`self.BPC_SpawnOnSolve`))))

(event `ShowBack`
  (`/Game/Environment/Gameplay/Collectibles/BPC_SpawnOnSolve.Show` (`self.BPC_SpawnOnSolve`)))

(event `self.ReceiveActorBeginOverlap`
  (params (OtherActor :type "Actor Object Reference"))
  (bind _asbp_t800_dora (cast `/Game/Gameplay/Player/BP_T800_Dora` OtherActor))
  (`/Engine/EditorBlueprintResources/StandardMacros.IncrementInt` (`/Game/Gameplay/Player/BP_T800_Dora.KeyCount` _asbp_t800_dora)
    (:`  `
      (`GameplayStatics.PlaySoundAtLocation` "/Game/Audio/Cue/SC_Mystical2.SC_Mystical2" (`self.K2_GetActorLocation`) (struct) 1.0 1.0 0.0 null null null null)
      (`self.K2_DestroyActor`))))

(fn `UserConstructionScript`)