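; Ofuda trap that pushes any overlapping LyokoCharacter along the actor's forward axis with a movement impulse scaled by Strengh.
; The first overlap also activates the Tornado effect and enlarges the Box component.
; Later overlaps keep applying the impulse until the Tornado system finishes and the actor destroys itself.
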(event `self.ReceiveActorBeginOverlap`
  (params (OtherActor :type "Actor Object Reference"))
  (bind (_returnvalue_location _returnvalue_rotation) (`KismetMathLibrary.BreakTransform` (`self.GetTransform`)))
  (bind _tornado (`self.Tornado`))
  (bind _aslyoko_character (cast `LyokoCharacter` OtherActor))
  (`CharacterMovementComponent.AddImpulse` (`Character.CharacterMovement` _aslyoko_character) (* (`KismetMathLibrary.GreaterGreater_VectorRotator` (1.0 0.0 0.0) _returnvalue_rotation) (`self.Strengh`)) false)
  (if (not (`self.IsTriggered`))
    (set `self.IsTriggered` true)
    (`ActorComponent.Activate` _tornado false)
    (add `NiagaraComponent.OnSystemFinished` _tornado (delegate `OnSystemFinished_Event`))
    (`SceneComponent.SetRelativeScale3D` (`self.Box`) (3.2 3.2 3.2))))

(event `OnSystemFinished_Event`
  (params (PSystem :type "NiagaraComponent Object Reference"))
  (`self.K2_DestroyActor`))

(fn `UserConstructionScript`)