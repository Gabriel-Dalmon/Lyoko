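; Explosive barrel trap that blows up when its health component fires its death event.
; On death, each LyokoCharacter overlapping the sphere gets a horizontal impulse away from the barrel, scaled by a blow strength, and takes damage.
; The barrel then spawns a Niagara explosion effect and sound at its location and destroys itself.
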(event `self.ReceiveBeginPlay`
  (add `HealthComponent.OnDeadEvent` (`self.Health`) (delegate `OnDeadEvent_Event`)))

(event `OnDeadEvent_Event`
  (bind _returnvalue (`self.K2_GetActorLocation`))
  (for _array_element (`PrimitiveComponent.GetOverlappingActors` (`self.Sphere`) "/Script/LyokoBase.LyokoCharacter")
    (bind _aslyoko_character (cast `LyokoCharacter` _array_element))
    (`CharacterMovementComponent.AddImpulse` (`Character.CharacterMovement` _aslyoko_character) (* (`KismetMathLibrary.Normal` (`KismetMathLibrary.MakeVector` (.x (- (`self.K2_GetActorLocation` _aslyoko_character) (`self.K2_GetActorLocation`))) (.y (- (`self.K2_GetActorLocation` _aslyoko_character) (`self.K2_GetActorLocation`))))) (`self.BlowStrengh`)) false)
    (`HealthComponent.TakeDamage` (`LyokoCharacterBase.HealthComponent` _aslyoko_character) (`self.Dmg`)))
  (`NiagaraFunctionLibrary.SpawnSystemAtLocation` "/Game/Environment/Explosion/NS_Explosion.NS_Explosion" _returnvalue (struct) (1.6 1.6 1.6))
  (`GameplayStatics.PlaySoundAtLocation` "/Game/Audio/Cue/SC_Explosion.SC_Explosion" _returnvalue (struct) 1.0 1.0 0.0 null null null null)
  (`self.K2_DestroyActor`))

(fn `UserConstructionScript`)