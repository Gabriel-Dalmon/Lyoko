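; BP_Altar is a gameplay altar that heals the BP_T800_Dora player to full health on primary interact.
; Overlapping a live altar stores the character and binds Heal to its interact event; leaving clears and unbinds it.
; Heal clears IsAlive to block later bindings, but the current binding lasts until overlap ends.
; Two SetVisibility hide calls are unwired, so the altar's visibility never changes here.
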(event `self.ReceiveActorBeginOverlap`
  (params (OtherActor :type "Actor Object Reference"))
  (if (`self.IsAlive`)
    (bind _asbp_t800_dora (cast `/Game/Gameplay/Player/BP_T800_Dora` OtherActor))
    (bind _output_get (set `self.CollisionningCharacter` _asbp_t800_dora))
    (add `/Game/Gameplay/Player/BP_T800_Dora.OnPlayerPrimaryInterract` _output_get (delegate `Heal`))))

(event `self.ReceiveActorEndOverlap`
  (params (OtherActor :type "Actor Object Reference"))
  (bind _asbp_t800_dora (cast `/Game/Gameplay/Player/BP_T800_Dora` OtherActor))
  (set `self.CollisionningCharacter` null)
  (remove `/Game/Gameplay/Player/BP_T800_Dora.OnPlayerPrimaryInterract` _asbp_t800_dora (delegate `Heal`)))

(event `Heal`
  (bind _healthcomponent (`LyokoCharacterBase.HealthComponent` (`self.CollisionningCharacter`)))
  (`HealthComponent.Heal` _healthcomponent (`HealthComponent.MaxHealth` _healthcomponent))
  (set `self.IsAlive` false))

(fn `UserConstructionScript`)