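; BP_PressureTrigger is an actionable pressure trigger that activates when an actor begins overlapping it and deactivates when an overlap ends.
; It notifies receivers through activated and deactivated events, which they bind or unbind via interface functions.
; Locally, each change swaps the mesh material and calls Solve or UnSolve on its win condition component.
; Overlaps are neither filtered nor counted, and GetState always returns false.
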(event `self.ReceiveActorBeginOverlap`
  (params (OtherActor :type "Actor Object Reference"))
  ;[0.6403 0.4605 1] Actionable State Detection
  (`self.OnActivated`)
  (`self.LocalOnActivated`))

(event `self.ReceiveActorEndOverlap`
  (params (OtherActor :type "Actor Object Reference"))
  ;[0.6403 0.4605 1] Actionable State Detection
  (`self.OnDeactivated`)
  (`self.LocalOnDeactivated`))

(event `self.BindEventToOnActivated`
  (params (Delegate :type "Delegate (by ref)"))
  ;[0.5214 1 0.4071] Interface Binding For Receivers
  (add `self.OnActivated` Delegate))

(event `self.UnbindEventFromOnActivated`
  (params (Delegate :type "Delegate (by ref)"))
  ;[0.5214 1 0.4071] Interface Binding For Receivers
  (remove `self.OnActivated` Delegate))

(event `self.BindEventToOnDeactivated`
  (params (Delegate :type "Delegate (by ref)"))
  ;[0.5214 1 0.4071] Interface Binding For Receivers
  (add `self.OnDeactivated` Delegate))

(event `self.UnbindEventFromOnDeactivated`
  (params (Delegate :type "Delegate (by ref)"))
  ;[0.5214 1 0.4071] Interface Binding For Receivers
  (remove `self.OnDeactivated` Delegate))

(fn `GetState`
  (returns (ReturnValue :type Boolean))
  (return false))

(fn `LocalOnActivated`
  (`PrimitiveComponent.SetMaterial` (`self.StaticMesh`) 0 "/Game/Environment/Gameplay/Actionables/MI_PressureTriggerActivated.MI_PressureTriggerActivated")
  (`/Game/Gameplay/BPC_WinCondition.Solve` (`self.BPC_WinCondition`)))

(fn `LocalOnDeactivated`
  (`PrimitiveComponent.SetMaterial` (`self.StaticMesh`) 0 "/Game/Environment/Gameplay/Actionables/M_PressureTrigger.M_PressureTrigger")
  (`/Game/Gameplay/BPC_WinCondition.UnSolve` (`self.BPC_WinCondition`)))

(fn `UserConstructionScript`)