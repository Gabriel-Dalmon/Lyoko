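; Pressure trigger that switches on while an overlapping BP_SaisenZone passes its CheckValidation test.
; Overlap stores the zone and binds to its coin amount changes, re-running the check on each change.
; Guarded SafeActivate and SafeDeactivate fire activation callbacks only on state changes; the mass threshold check is unused.
; End overlap deactivates, but clears the zone reference before unbinding, so the unbind targets None.
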(event `self.ReceiveActorBeginOverlap`
  (params (OtherActor :type "Actor Object Reference"))
  (bind _asbp_saisen_zone (cast `/Game/Environment/Gameplay/Saisen/BP_SaisenZone` OtherActor))
  (set `self.TriggeringObject` _asbp_saisen_zone)
  (`self.CheckPressureState`)
  ; If the actor is a Saisen, we bind on coin amount change event
  (add `/Game/Environment/Gameplay/Saisen/BP_SaisenZone.OnCoinAmountChange` (`self.TriggeringObject`) (delegate `OnMassChanged_Event`)))

(event `OnMassChanged_Event`
  ; If mass changed while overlap is active
  (`self.CheckPressureState`))

(event `self.ReceiveActorEndOverlap`
  (params (OtherActor :type "Actor Object Reference"))
  (cast `/Game/Environment/Gameplay/Saisen/BP_SaisenZone` OtherActor)
  (set `self.TriggeringObject` null)
  (`self.SafeDeactivate`)
  ; If we stop overlapping with a saisen, we want to unbind our functions
  (remove `/Game/Environment/Gameplay/Saisen/BP_SaisenZone.OnCoinAmountChange` (`self.TriggeringObject`) (delegate `OnMassChanged_Event`)))

(fn `CheckPressureState`
  (bind _isvalidated (`/Game/Environment/Gameplay/Saisen/BP_SaisenZone.CheckValidation` (`self.TriggeringObject`)))
  (if _isvalidated
    (`self.SafeActivate`)
    (else
      (`self.SafeDeactivate`))))

(fn `SafeActivate`
  (if (not (`self.IsActive`))
    (set `self.IsActive` true)
    (`self.OnActivated`)
    (`self.LocalOnActivated`)))

(fn `SafeDeactivate`
  (if (`self.IsActive`)
    (`self.OnDeactivated`)
    (`self.LocalOnDeactivated`)
    (set `self.IsActive` false)))

(fn `UserConstructionScript`
  (`parent.UserConstructionScript`))