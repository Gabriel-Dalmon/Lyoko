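; BP_DialogueLauncher is a one-shot trigger actor that shows a timed dialogue widget when BP_T800_Dora overlaps it.
; The overlap calls the CallDialogue event, which destroys the Box component, then creates the Dialogue widget class for player 0 and adds it to the viewport.
; After a Delay of Duration, the widget is removed from the screen, while the actor itself remains.
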(event `self.ReceiveActorBeginOverlap`
  (params (OtherActor :type "Actor Object Reference"))
  (cast `/Game/Gameplay/Player/BP_T800_Dora` OtherActor)
  (`self.CallDialogue`))

(event `CallDialogue`
  (`ActorComponent.K2_DestroyComponent` (`self.Box`))
  (bind _returnvalue (`|CreateWidget` (`self.Dialogue`) (`GameplayStatics.GetPlayerController` 0)))
  (bind _output_get (set `self.InstanciatedWidget` _returnvalue))
  (`UserWidget.AddToViewport` _output_get 0)
  (`KismetSystemLibrary.Delay` (`self.Duration`))
  (`Widget.RemoveFromParent` (`self.InstanciatedWidget`)))

(fn `UserConstructionScript`)