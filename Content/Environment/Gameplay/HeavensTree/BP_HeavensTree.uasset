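; BP_HeavensTree is a floor-exit actor that appears when a room is over and completes the floor when touched.
; On BeginPlay it binds to the room-over event of each BP_RoomBase overlapping its Box, then hides through BPCSpawnOnSolve.
; The room-over event shows it again through that component.
; An overlap by BP_T800_Dora calls EventOnFloorComplet on the top-down player controller, with no room-state check.
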(event `self.ReceiveBeginPlay`
  (for _array_element (`PrimitiveComponent.GetOverlappingActors` (`self.Box`) "/Game/Gameplay/Rooms/BP_RoomBase.BP_RoomBase_C")
    (bind _asbp_room_base (cast `/Game/Gameplay/Rooms/BP_RoomBase` _array_element))
    (add `/Game/Gameplay/Rooms/BP_RoomBase.OnRoomOver` _asbp_room_base (delegate `ShowBack`)))
  (`/Game/Environment/Gameplay/Collectibles/BPC_SpawnOnSolve.Hide` (`self.BPC_SpawnOnSolve`)))

(event `ShowBack`
  (`/Game/Environment/Gameplay/Collectibles/BPC_SpawnOnSolve.Show` (`self.BPC_SpawnOnSolve`)))

(event `self.ReceiveActorBeginOverlap`
  (params (OtherActor :type "Actor Object Reference"))
  (cast `/Game/Gameplay/Player/BP_T800_Dora` OtherActor)
  (bind _asbp_top_down_player_controller (cast `/Game/Gameplay/Player/BP_TopDownPlayerController` (`GameplayStatics.GetPlayerController` 0)))
  (`/Game/Gameplay/Player/BP_TopDownPlayerController.EventOnFloorComplet` _asbp_top_down_player_controller))

(fn `UserConstructionScript`)