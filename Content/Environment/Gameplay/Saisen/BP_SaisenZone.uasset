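; BP_SaisenZone is an interaction zone for a saisen box that players can drag and fill with coins.
; While BP_T800_Dora overlaps it, the player's three interact dispatchers are bound to grab/release, add coin and remove coin.
; Coins transfer to and from the player's count, firing OnCoinAmountChange.
; Dragging uses the player's PhysicsHandle, updated on Tick, with speed reduced by coins held at grab time and grabbing blocked at StopMovingAtCount.
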(event `self.ReceiveBeginPlay`
  (set `self.CurrentCoinAmount` (`self.BaseCoinAmount`))
  (`SceneComponent.SetVisibility` (`self.Commands`) false false))

(event `self.ReceiveActorBeginOverlap`
  (params (OtherActor :type "Actor Object Reference"))
  ; Player is close, we bind our functions
  (bind _asbp_t800_dora (cast `/Game/Gameplay/Player/BP_T800_Dora` OtherActor))
  (set `self.CollisionningCharacter` _asbp_t800_dora)
  (add `/Game/Gameplay/Player/BP_T800_Dora.OnPlayerPrimaryInterract` _asbp_t800_dora (delegate `MoveSaisen`))
  (add `/Game/Gameplay/Player/BP_T800_Dora.OnPlayerSecondaryInterract` _asbp_t800_dora (delegate `AddCoin`))
  (add `/Game/Gameplay/Player/BP_T800_Dora.OnPlayerTernaryInteract` _asbp_t800_dora (delegate `RemoveCoin`))
  (`SceneComponent.SetVisibility` (`self.Commands`) (`self.ShowCommands`) false))

(event `self.ReceiveActorEndOverlap`
  (params (OtherActor :type "Actor Object Reference"))
  ; Player gets further, we unbind our functions
  (bind _asbp_t800_dora (cast `/Game/Gameplay/Player/BP_T800_Dora` OtherActor))
  (set `self.CollisionningCharacter` null)
  (remove `/Game/Gameplay/Player/BP_T800_Dora.OnPlayerPrimaryInterract` _asbp_t800_dora (delegate `MoveSaisen`))
  (remove `/Game/Gameplay/Player/BP_T800_Dora.OnPlayerSecondaryInterract` _asbp_t800_dora (delegate `AddCoin`))
  (remove `/Game/Gameplay/Player/BP_T800_Dora.OnPlayerTernaryInteract` _asbp_t800_dora (delegate `RemoveCoin`))
  (`SceneComponent.SetVisibility` (`self.Commands`) false false))

(event `MoveSaisen`
  ; Call SaisenCore's functions
  (if (< (`self.CurrentCoinAmount`) (`self.StopMovingAtCount`))
    (`self.FlipFlopGrab`)
    (else
      (`KismetSystemLibrary.PrintString` "Should informe the player that saisen is too heavy"))))

(event `AddCoin`
  ; Call SaisenCore's functions
  (if (>= (`/Game/Gameplay/Player/BP_T800_Dora.CoinsCount` (`self.CollisionningCharacter`)) 1)
    (`/Game/Gameplay/Player/BP_T800_Dora.UpdateCoinsCount` (`self.CollisionningCharacter`) -1)
    (`/Engine/EditorBlueprintResources/StandardMacros.IncrementInt` (`self.CurrentCoinAmount`)
      (:`  `
        (`self.OnCoinAmountChange` :!label _label)))))

(event `RemoveCoin`
  ; Call SaisenCore's functions
  (if (>= (`self.CurrentCoinAmount`) 1)
    (`/Game/Gameplay/Player/BP_T800_Dora.UpdateCoinsCount` (`self.CollisionningCharacter`) 1)
    (`/Engine/EditorBlueprintResources/StandardMacros.DecrementInt` (`self.CurrentCoinAmount`)
      (:`  `
        (goto _label)))))

(event `self.ReceiveTick`
  (params (DeltaSeconds :type "Float (single-precision)"))
  (bind _collisionningcharacter (`self.CollisionningCharacter`))
  (if (and (`self.IsDraggedByPlayer`) (`KismetSystemLibrary.IsValid` _collisionningcharacter))
    (`/Game/Gameplay/Player/BP_T800_Dora.MovePhysicsHandleLocation` (`self.CollisionningCharacter`) (`self.K2_GetActorLocation` _collisionningcharacter))))

(fn `FlipFlopGrab`
  (bind _returnvalue (+ (`self.StopMovingAtCount`) 1))
  (bind _output_get (set `self.IsDraggedByPlayer` (not (`self.IsDraggedByPlayer`))))
  (if _output_get
    (`PhysicsHandleComponent.GrabComponentAtLocation` (`/Game/Gameplay/Player/BP_T800_Dora.PhysicsHandle` (`self.CollisionningCharacter`)) (`self.StaticMesh`) "None" (`self.K2_GetActorLocation` (`self.CollisionningCharacter`)))
    (`/Game/Gameplay/Player/BP_T800_Dora.SetSpeedByMultiplicator` (`self.CollisionningCharacter`) (* (/ 1.0 (`KismetMathLibrary.Conv_IntToDouble` _returnvalue)) (`KismetMathLibrary.Conv_IntToDouble` (- _returnvalue (+ (`self.CurrentCoinAmount`) 1)))))
    (return)
    (else
      (set `self.IsDraggedByPlayer` false)
      (`PhysicsHandleComponent.ReleaseComponent` (`/Game/Gameplay/Player/BP_T800_Dora.PhysicsHandle` (`self.CollisionningCharacter`)))
      (`/Game/Gameplay/Player/BP_T800_Dora.SetSpeedByMultiplicator` (`self.CollisionningCharacter`) 1.0))))

(fn `UserConstructionScript`)