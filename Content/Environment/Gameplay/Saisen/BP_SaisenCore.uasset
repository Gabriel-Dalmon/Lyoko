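; BP_SaisenCore is the core of a saisen (offering box) that holds coins and uses their count as its mass.
; AddCoin takes one coin from the passed object when it has any, and RemoveCoin gives one back when the box is not empty.
; Each transfer updates Mass from CoinAmount and calls coin-amount and mass change notifications, while BeginPlay initializes Mass from the starting CoinAmount.
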(event `self.ReceiveBeginPlay`
  (set `self.Mass` (`self.CoinAmount`)))

(fn `AddCoin`
  (params (NewParam :type "/Game/Gameplay/Player/BP_T800_Dora Object Reference"))
  (if (>= (`/Game/Gameplay/Player/BP_T800_Dora.CoinsCount` NewParam) 1)
    (`/Game/Gameplay/Player/BP_T800_Dora.UpdateCoinsCount` NewParam -1)
    (bind _result (`/Engine/EditorBlueprintResources/StandardMacros.IncrementInt` (`self.CoinAmount`))
      (:`  `
        (set `self.Mass` _result)
        (`self.OnCoinAmountChange`)
        (`self.OnMassChanged`)
        (return)))))

(fn `RemoveCoin`
  (params (NewParam :type "/Game/Gameplay/Player/BP_T800_Dora Object Reference"))
  (if (>= (`self.CoinAmount`) 1)
    (`/Game/Gameplay/Player/BP_T800_Dora.UpdateCoinsCount` NewParam 1)
    (bind _result (`/Engine/EditorBlueprintResources/StandardMacros.DecrementInt` (`self.CoinAmount`))
      (:`  `
        (set `self.Mass` _result)
        (`self.OnCoinAmountChange`)
        (`self.OnMassChanged`)
        (return)))))

(fn `UserConstructionScript`)