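; BP_Corridor is a corridor piece that switches the roof visibility of adjacent corridors as the BP_T800_Dora player moves through it.
; One tick after BeginPlay, it caches the corridors overlapping its Box as neighbours.
; Player overlap sets an occupancy flag, fires enter/exit calls and toggles neighbour roofs on or off.
; On exit, neighbours still holding the player are skipped.
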(event `self.ReceiveBeginPlay`
  (`KismetSystemLibrary.DelayUntilNextTick`)
  (for _array_element (`PrimitiveComponent.GetOverlappingActors` (`self.Box`) "BP_Corridor_C")
    (bind _asbp_corridor (cast `/Game/Environment/Gameplay/BP_Corridor` _array_element))
    (`KismetArrayLibrary.Array_Add` (`self.Neighbour`) _asbp_corridor)))

(event `self.ReceiveActorBeginOverlap`
  (params (OtherActor :type "Actor Object Reference"))
  (cast `/Game/Gameplay/Player/BP_T800_Dora` OtherActor)
  (set `self.IsPlayerInCorridor` true)
  (`self.OnEnter`)
  (for _array_element (`self.Neighbour`)
    (`/Game/Environment/Gameplay/BP_MainRoof.ToggleVisibilityOn` (`/Game/Environment/Gameplay/BP_Corridor.Roof` _array_element))))

(event `self.ReceiveActorEndOverlap`
  (params (OtherActor :type "Actor Object Reference"))
  (cast `/Game/Gameplay/Player/BP_T800_Dora` OtherActor)
  (set `self.IsPlayerInCorridor` false)
  (`self.OnExit`)
  (for _array_element (`self.Neighbour`)
    (if (not (`/Game/Environment/Gameplay/BP_Corridor.IsPlayerInCorridor` _array_element))
      (`/Game/Environment/Gameplay/BP_MainRoof.ToggleVisibilityOff` (`/Game/Environment/Gameplay/BP_Corridor.Roof` _array_element)))))

(fn `UserConstructionScript`)