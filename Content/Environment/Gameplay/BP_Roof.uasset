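; BP_Roof is a roof actor whose visibility can be toggled by animating its material opacity.
; On BeginPlay it creates a dynamic material instance for StaticMesh1's first material slot and sets its Opacity parameter to fully opaque.
; ToggleVisibilityOn plays a Timeline that writes its curve value to Opacity on each update, and ToggleVisibilityOff reverses that same Timeline.
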(event `self.ReceiveBeginPlay`
  (bind _returnvalue (`KismetMaterialLibrary.CreateDynamicMaterialInstance` (`PrimitiveComponent.GetMaterial` (`self.StaticMesh1`) 0)))
  (bind _output_get (set `self.DynamicMaterialInstance` _returnvalue))
  (`PrimitiveComponent.SetMaterial` (`self.StaticMesh1`) 0 _output_get)
  (`MaterialInstanceDynamic.SetScalarParameterValue` (`self.DynamicMaterialInstance`) "Opacity" 1.0))

(event `ToggleVisibilityOn`
  (bind (_direction _updateopacity) (`Timeline|Timeline` :!label _label)
    (:`Update`
      (`MaterialInstanceDynamic.SetScalarParameterValue` (`self.DynamicMaterialInstance`) "Opacity" _updateopacity))))

(event `ToggleVisibilityOff`
  (goto _label :!via `Reverse`))

(fn `UserConstructionScript`)