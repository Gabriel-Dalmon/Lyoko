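; BP_AttackOmamori is an attack charm collectible that boosts the damage of the BP_T800_Dora character who picks it up.
; On pickup it casts the pickuper to BP_T800_Dora and multiplies that character's AttackDamageMultiplicator by its own AttackMultiplicator, so repeated pickups compound.
; It stubs out the carry and steal functions, always reporting that it is not carried and cannot be stolen.
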(event `self.OnPickedUp`
  (params (Pickuper :type "Pickuper Interface (by ref)"))
  (bind _asbp_t800_dora (cast `/Game/Gameplay/Player/BP_T800_Dora` Pickuper))
  (set `/Game/Gameplay/Player/BP_T800_Dora.AttackDamageMultiplicator` (* (`/Game/Gameplay/Player/BP_T800_Dora.AttackDamageMultiplicator` _asbp_t800_dora) (`self.AttackMultiplicator`)) _asbp_t800_dora))

(fn `CanBeStolen`
  (params (Stealer :type "Pickuper Interface (by ref)"))
  (returns (ReturnValue :type Boolean))
  (return false))

(fn `GetCarrier`
  (returns (ReturnValue :type "Pickuper Interface"))
  (return null))

(fn `IsCarried`
  (returns (ReturnValue :type Boolean))
  (return false))

(fn `UserConstructionScript`)