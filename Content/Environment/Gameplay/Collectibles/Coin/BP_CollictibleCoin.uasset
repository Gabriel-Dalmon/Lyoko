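; A collectible coin actor that BP_T800_Dora picks up by overlapping it.
; On overlap with that character it adds one to the coin count through UpdateCoinsCount, plays the SC_GrabCoin sound at its location and destroys itself.
; IsCarried, GetCarrier and CanBeStolen are stubs that report the coin as never carried, without a carrier and not stealable.
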(event `self.ReceiveActorBeginOverlap`
  (params (OtherActor :type "Actor Object Reference"))
  (bind _asbp_t800_dora (cast `/Game/Gameplay/Player/BP_T800_Dora` OtherActor))
  (`/Game/Gameplay/Player/BP_T800_Dora.UpdateCoinsCount` _asbp_t800_dora 1)
  (`GameplayStatics.PlaySoundAtLocation` "/Game/Audio/Cue/SC_GrabCoin.SC_GrabCoin" (`self.K2_GetActorLocation`) (struct) 1.0 1.0 0.0 null null null null)
  (`self.K2_DestroyActor`))

(fn `CanBeStolen`
  (params (Stealer :type "Pickuper Interface (by ref)"))
  (returns (ReturnValue :type Boolean))
  (return false))

(fn `GetCarrier`
  (returns (ReturnValue :type "Pickuper Interface"))
  (return null))

(fn `IsCarried`
  (returns (ReturnValue :type Boolean))
  (return false))

(fn `UserConstructionScript`)