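; Health omamori collectible that permanently raises the Dora character's max health on overlap.
; Optionally hides on spawn through its spawn-on-solve component and reappears when an overlapping room fires its room-over event, bound a tick after BeginPlay.
; On pickup it removes its sphere and idle visual, attaches to the player, plays a sound and Niagara burst, then destroys itself when the effect finishes.
; Carry and steal queries always report false.
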(event `self.ReceiveBeginPlay`
  (if (`self.SpawnOnRoomOver`)
    (`KismetSystemLibrary.DelayUntilNextTick`)
    (for _array_element (`PrimitiveComponent.GetOverlappingActors` (`self.Sphere`) "/Game/Gameplay/Rooms/BP_RoomBase.BP_RoomBase_C")
      (bind _asbp_room_base (cast `/Game/Gameplay/Rooms/BP_RoomBase` _array_element))
      (add `/Game/Gameplay/Rooms/BP_RoomBase.OnRoomOver` _asbp_room_base (delegate `ShowBack`)))
    (`/Game/Environment/Gameplay/Collectibles/BPC_SpawnOnSolve.Hide` (`self.BPC_SpawnOnSolve`))))

(event `ShowBack`
  (`/Game/Environment/Gameplay/Collectibles/BPC_SpawnOnSolve.Show` (`self.BPC_SpawnOnSolve`)))

(event `self.ReceiveActorBeginOverlap`
  (params (OtherActor :type "Actor Object Reference"))
  (bind _bonusfx (`self.BonusFx`))
  (bind _asbp_t800_dora (cast `/Game/Gameplay/Player/BP_T800_Dora` OtherActor))
  (`HealthComponent.AddMaxHealth` (`LyokoCharacterBase.HealthComponent` _asbp_t800_dora) (`self.BonusHealth`))
  (`ActorComponent.K2_DestroyComponent` (`self.Sphere`))
  (`ActorComponent.K2_DestroyComponent` (`self.OmamoriIdle`))
  (`ActorComponent.Activate` _bonusfx false)
  (add `NiagaraComponent.OnSystemFinished` _bonusfx (delegate `OnNiagaraFinished`))
  (`self.K2_AttachToActor` _asbp_t800_dora "None" "SnapToTarget" "KeepRelative" "KeepRelative")
  (`GameplayStatics.PlaySoundAtLocation` "/Game/Audio/Cue/SC_Mystical2.SC_Mystical2" (`self.K2_GetActorLocation`) (struct) 1.0 1.0 0.0 null null null null))

(event `OnNiagaraFinished`
  (params (PSystem :type "NiagaraComponent Object Reference"))
  (`self.K2_DestroyActor`))

(fn `CanBeStolen`
  (params (Stealer :type "Pickuper Interface (by ref)"))
  (returns (ReturnValue :type Boolean))
  (return false))

(fn `GetCarrier`
  (returns (ReturnValue :type "Pickuper Interface"))
  (return null))

(fn `IsCarried`
  (returns (ReturnValue :type Boolean))
  (return false))

(fn `UserConstructionScript`)