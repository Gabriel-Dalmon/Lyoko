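; BP_Door is a sliding double door that responds to a set of linked Actionable objects.
; BeginPlay binds to each valid Actionable's activation messages and calls the open event; a counter then triggers opening when all are active and closing when one drops out.
; A speed-scaled Timeline slides both panels, reversing to close, with a sound each way.
; Its collision Box is destroyed when added to a room pool, avoiding needless collision tests.
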(event `self.ReceiveBeginPlay`
  ; BeginPlay
  (`|ExecutionSequence`
    (:`then_0`
      ;; Door specific initialization
      (`TimelineComponent.SetPlayRate` (`self.Timeline`) (`self.DoorAnimationSpeed`)))
    (:`then_1`
      (for _array_element (`self.Actionables`)
        (if (`self.IsActionableValid` _array_element)
          (`|ExecutionSequence`
            (:`then_0`
              ;; Bind Receiver to Actionable "OnActivated" event
              (message `Actionable.BindEventToOnActivated` _array_element (delegate `/Game/Environment/Gameplay/Interfaces/Receiver.OnSingleActionableActivated`)))
            (:`then_1`
              ;; Bind Receiver to Actionable "OnDeactivated" event
              (message `Actionable.BindEventToOnDeactivated` _array_element (delegate `/Game/Environment/Gameplay/Interfaces/Receiver.OnSingleActionableDeactivated`)))))))
    (:`then_2`
      (`self.Open_Event`))))

(event `/Game/Environment/Gameplay/Interfaces/Receiver.OnSingleActionableActivated`
  ; BeginPlay
  ;; Bind Receiver to Actionable "OnActivated" event
  (`self.OnSingleActionableActivated_Implementation`))

(event `/Game/Environment/Gameplay/Interfaces/Receiver.OnSingleActionableDeactivated`
  ; BeginPlay
  ;; Bind Receiver to Actionable "OnDeactivated" event
  (`self.OnSingleActionableDeactivated_Implementation`))

(event `/Game/Environment/Gameplay/Interfaces/Receiver.OnAllActionablesActiveCancelled`
  ; Call door specific logic
  (`self.Close_Event`))

(event `OnAddedToRoomPool`
  ; Optimization to avoid useless collision tests
  (`ActorComponent.K2_DestroyComponent` (`self.Box`)))

(event `/Game/Environment/Gameplay/Interfaces/Receiver.OnAllActionablesActive`
  ; Call door specific logic
  (`self.Open_Event`))

(event `Open_Event`
  ; Play Door animations
  (`GameplayStatics.PlaySound2D` "/Game/Audio/Cue/SC_DoorOpening.SC_DoorOpening" 1.0 1.0 0.0 null null)
  (bind (_direction _rightdoorx _leftdoorx) (`Timeline|Timeline` :!label _label)
    (:`Update`
      (`|ExecutionSequence`
        (:`then_0`
          (`SceneComponent.K2_SetRelativeLocation` (`self.RightDoor`) (`KismetMathLibrary.MakeVector` 0.0 _rightdoorx) false false))
        (:`then_1`
          (`SceneComponent.K2_SetRelativeLocation` (`self.LeftDoor`) (`KismetMathLibrary.MakeVector` 0.0 _leftdoorx) false false))))))

(event `Close_Event`
  ; Play Door animations
  (`GameplayStatics.PlaySound2D` "/Game/Audio/Cue/SC_DoorOpening.SC_DoorOpening" 1.0 1.0 0.0 null null)
  (goto _label :!via `Reverse`))

(fn `BindToOnActivated`)

(fn `OnSingleActionableActivated_Implementation`
  (`/Engine/EditorBlueprintResources/StandardMacros.IncrementInt` (`self.ActiveActionablesCount`)
    (:`  `
      (if (`self.AreAllActionablesActive`)
        (`self.OnAllActionablesActive`)))))

(fn `OnSingleActionableDeactivated_Implementation`
  (`/Engine/EditorBlueprintResources/StandardMacros.DecrementInt` (`self.ActiveActionablesCount`)
    (:`  `
      (if (`self.IsOnlyOneActionableDeactivated`)
        (`self.OnAllActionablesActiveCancelled`)))))

(fn `UserConstructionScript`)