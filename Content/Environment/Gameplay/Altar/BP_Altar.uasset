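; BP_Altar is an altar where the overlapping T800_Dora character can pray to heal to full health.
; Overlap binds Use to the character's secondary interact while the altar is alive, and end overlap unbinds it.
; Use locks movement, heals, marks the altar dead, and triggers audio, music ducking and a Niagara energy wave.
; A timeline animates inner and outer lights, then restores the sound mix and unlocks movement.
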(event `self.ReceiveActorBeginOverlap`
  (params (OtherActor :type "Actor Object Reference"))
  (if (`self.IsAlive`)
    (bind _asbp_t800_dora (cast `/Game/Gameplay/Player/BP_T800_Dora` OtherActor))
    (bind _output_get (set `self.CollisionningCharacter` _asbp_t800_dora))
    (add `/Game/Gameplay/Player/BP_T800_Dora.OnPlayerSecondaryInterract` _output_get (delegate `Use`))))

(event `self.ReceiveActorEndOverlap`
  (params (OtherActor :type "Actor Object Reference"))
  (bind _asbp_t800_dora (cast `/Game/Gameplay/Player/BP_T800_Dora` OtherActor))
  (set `self.CollisionningCharacter` null)
  (remove `/Game/Gameplay/Player/BP_T800_Dora.OnPlayerSecondaryInterract` _asbp_t800_dora (delegate `Use`)))

(event `Use`
  (bind _collisionningcharacter (`self.CollisionningCharacter`))
  (bind _healthcomponent (`LyokoCharacterBase.HealthComponent` _collisionningcharacter))
  (`/Game/Gameplay/Player/BP_T800_Dora.LockMovements` _collisionningcharacter)
  (`HealthComponent.Heal` _healthcomponent (`HealthComponent.MaxHealth` _healthcomponent))
  (`/Game/Gameplay/Player/BP_T800_Dora.Event OnPrayer` _collisionningcharacter)
  (set `self.IsAlive` false)
  (`AudioComponent.Play` (`self.AudioEmitter`) 0.0)
  (`GameplayStatics.PushSoundMixModifier` "/Game/Audio/SCM_DuckMusic.SCM_DuckMusic")
  (`NiagaraFunctionLibrary.SpawnSystemAtLocation` "/Game/Environment/Gameplay/Shockwave/NS_EnergyWave.NS_EnergyWave" (`self.K2_GetActorLocation`) (struct) (5.0 5.0 5.0))
  (bind (_direction _innrelightintensity _outerlightintensity) (`Timeline|Lights`)
    (:`Update`
      (`LightComponent.SetIntensity` (`self.InnerLight`) _innrelightintensity)
      (`LightComponent.SetIntensity` (`self.OuterLight`) _outerlightintensity))
    (:`Finished`
      (`GameplayStatics.PopSoundMixModifier` "/Game/Audio/SCM_DuckMusic.SCM_DuckMusic")
      (`/Game/Gameplay/Player/BP_T800_Dora.UnlockMovements` (`self.CollisionningCharacter`)))))

(fn `UserConstructionScript`)