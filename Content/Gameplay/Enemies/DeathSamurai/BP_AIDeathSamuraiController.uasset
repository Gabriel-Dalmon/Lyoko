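; AI controller for the Death Samurai enemy that drives its behavior state through the Blackboard.
; Perception updates set player-tagged actors as target and switch state, and switch again when the current target is lost.
; Perceived and forgotten events track a threat actor and perceived flag.
; Blackboard state changes are forwarded to the pawn with previous and new states, and a helper exposes the stored weapon.
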(event `self.AIPerception.OnTargetPerceptionUpdated`
  (params (Actor :type "Actor Object Reference") (Stimulus :type "AIStimulus Structure"))
  ; AIPerception Events
  (if Stimulus_bSuccessfullySensed
    ;; On Potential Target Perceived
    (if (`self.IsPotentialTarget` Actor)
      ;;;[0.8958 0.2286 0.3036 0.5] On Valid Target Perceived
      (`self.SetTargetActor` Actor)
      (`self.Set Behavior State` "NewEnumerator3"))
    (else
      ;; On Target Lost
      (if (`self.IsCurrentTarget` Actor)
        (`self.Set Behavior State` "NewEnumerator2")))))

(event `self.OnPerceived`
  (params (`Threat Actor` :type "Actor Object Reference"))
  ; Threaten Logic
  (`self.SetThreatActor` `Threat Actor`)
  (set `self.IsPerceived` true))

(event `self.OnForgotten`
  (params (`Threat Actor` :type "Actor Object Reference"))
  ; Threaten Logic
  (if (== `Threat Actor` (`self.GetCurrentThreatActor`))
    (`self.SetThreatActor` null)
    (set `self.IsPerceived` false)))

(event `self.OnBehaviourStateChanged`
  (params (ChangedKeyName :type Name))
  (bind _returnvalue (cast `/Game/Gameplay/Enemies/DeathSamurai/EDeathSamuraiStates` (`BlackboardComponent.GetValueAsEnum` (`self.BlackboardComponent`) ChangedKeyName)))
  (if (`|EnumInequality` (`self.PreviousState`) _returnvalue)
    (bind _asbp_death_samurai (cast `/Game/Gameplay/Enemies/DeathSamurai/BP_DeathSamurai` (`self.K2_GetPawn`)))
    (`/Game/Gameplay/Enemies/DeathSamurai/BP_DeathSamurai.OnAIStateChanged` _asbp_death_samurai (`self.PreviousState`) _returnvalue)
    (set `self.PreviousState` _returnvalue)))

(fn `GetCurrentThreatActor`
  (returns (`Threat Actor` :type "Object Object Reference"))
  (return (`BlackboardComponent.GetValueAsObject` (`self.BlackboardComponent`) (`self.ThreatActorKey`))))

(fn `GetWeapon`
  (returns (Weapon :type "WeaponBase Object Reference") (HasWeapon :type Boolean))
  (bind _asweapon_base (cast `WeaponBase` (`BlackboardComponent.GetValueAsObject` (`self.BlackboardComponent`) (`self.Weapon Key`)))
    (:`then`
      (return _asweapon_base true))
    (:`CastFailed`
      (return null false))))

(fn `IsCurrentTarget`
  (params (Actor :type "Object Object Reference"))
  (returns (ReturnValue :type Boolean))
  (return (== Actor (`BlackboardComponent.GetValueAsObject` (`self.BlackboardComponent`) (`self.TargetActorKey`)))))

(fn `IsPotentialTarget`
  (params (Actor :type "Actor Object Reference"))
  (returns (ReturnValue :type Boolean))
  (return (`self.ActorHasTag` Actor (`self.PlayerTag`))))

(fn `Set Behavior State`
  (params (`New State` :type "/Game/Gameplay/Enemies/DeathSamurai/EDeathSamuraiStates Enum" :default "NewEnumerator0"))
  (`BlackboardComponent.SetValueAsEnum` (`self.BlackboardComponent`) (`self.StateKey`) `New State`))

(fn `SetTargetActor`
  (params (`Target Actor` :type "Object Object Reference"))
  (`BlackboardComponent.SetValueAsObject` (`self.BlackboardComponent`) (`self.TargetActorKey`) `Target Actor`))

(fn `SetThreatActor`
  (params (ThreatActor :type "Object Object Reference"))
  (`BlackboardComponent.SetValueAsObject` (`self.BlackboardComponent`) (`self.ThreatActorKey`) ThreatActor))

(fn `UserConstructionScript`)