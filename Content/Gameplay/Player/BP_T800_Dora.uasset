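; Top-down player character that spawns with a kunai weapon and handles dash, throw attack, prayer, death, coins and room combat state.
; Actions gate each other through movement, look, dash and attack locks, partly routed via the player controller.
; Dash is a swept timeline lerp along last input, with a cooldown.
; A Quartz clock applies pending slow/fast music switches on bar boundaries through audio parameters, while a timeline adjusts footstep volume.
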(event `self.ReceiveBeginPlay`
  (bind _returnvalue (`|SpawnActorFromClass` "/Game/Gameplay/Items/BP_KunaiWeapon.BP_KunaiWeapon_C" (`KismetMathLibrary.MakeTransform` (0.0 0.0 0.0)) "Undefined" "MultiplyWithRoot" null null))
  (`Pickuper.Pickup` _returnvalue)
  (set `self.BaseMouSpeed` (`CharacterMovementComponent.MaxWalkSpeed` (`self.CharacterMovement`)))
  ; Quartz Clock setup
  (bind _returnvalue_2 (`QuartzSubsystem.CreateNewClock` (subsystem `QuartzSubsystem`) "MusicClock" (make `QuartzClockSettings` (make `QuartzTimeSignature` 4)) false true))
  (bind _clockhandle (`QuartzClockHandle.SetBeatsPerMinute` :`self` _returnvalue_2 :`BeatsPerMinute` 130.0))
  (bind _output_get (set `self.ClockHandle` _clockhandle))
  (bind _clockhandle_2 (`QuartzClockHandle.StartClock` _output_get))
  (`QuartzClockHandle.SubscribeToQuantizationEvent` _clockhandle_2 "Bar" (delegate `LookForMusicChange`))
  (`AudioComponent.Play` (`self.MusicEmitter`) 0.0)
  (set `self.PreviousTrack` "NewEnumerator0"))

(event `EnhancedInput|/Game/Inputs/IA_PrimaryAction`
  (params (ActionValue :type Boolean) (ElapsedSeconds :type "Float (double-precision)") (TriggeredSeconds :type "Float (double-precision)") (InputAction :type "InputAction Object Reference" :default "/Game/Inputs/IA_PrimaryAction.IA_PrimaryAction"))
  ; Input Mapping
  (:`Triggered`
    (`self.OnPlayerPrimaryInterract`)))

(event `LookForMusicChange`
  (params (ClockName :type Name) (QuantizationType :type "EQuartzCommandQuantization Enum" :default "Bar") (NumBars :type Integer) (Beat :type Integer) (BeatFraction :type "Float (single-precision)"))
  (bind _mustchangetrack (`self.MustChangeTrack`))
  (bind _musicemitter (`self.MusicEmitter`))
  (bind _musicemitter_2 (`self.MusicEmitter`))
  ; Change music callback
  (if _mustchangetrack
    (set `self.MustChangeTrack` (not _mustchangetrack))
    (switch `/Game/Audio/EN_Track` (`self.PreviousTrack`)
      (:`NewEnumerator0`
        (set `self.PreviousTrack` "NewEnumerator1")
        (`AudioComponent.SetIntParameter` _musicemitter_2 "TrackID" (`KismetMathLibrary.Conv_ByteToInt` (`self.PreviousTrack`)))
        (`AudioParameterControllerInterface.SetTriggerParameter` _musicemitter_2 "TriggerChange")
        ;; The Timeline duration is calculated from the current music settings
        (bind (_direction _footstepvolume) (`Timeline|Footsteps volume` :!via `Reverse` :!label _label)
          (:`Update`
            (set `self.FootstepsVolume` _footstepvolume))))
      (:`NewEnumerator1`
        (set `self.PreviousTrack` "NewEnumerator0")
        (`AudioComponent.SetIntParameter` _musicemitter "TrackID" (`KismetMathLibrary.Conv_ByteToInt` (`self.PreviousTrack`)))
        (`AudioParameterControllerInterface.SetTriggerParameter` _musicemitter "TriggerChange")
        (goto _label)))))

(event `EnhancedInput|/Game/Inputs/IA_SecondaryAction`
  (params (ActionValue :type Boolean) (ElapsedSeconds :type "Float (double-precision)") (TriggeredSeconds :type "Float (double-precision)") (InputAction :type "InputAction Object Reference" :default "/Game/Inputs/IA_SecondaryAction.IA_SecondaryAction"))
  ; Input Mapping
  (:`Triggered`
    (`self.OnPlayerSecondaryInterract`)))

(event `EnhancedInput|/Game/Inputs/IA_TernaryAction`
  (params (ActionValue :type Boolean) (ElapsedSeconds :type "Float (double-precision)") (TriggeredSeconds :type "Float (double-precision)") (InputAction :type "InputAction Object Reference" :default "/Game/Inputs/IA_TernaryAction.IA_TernaryAction"))
  ; Input Mapping
  (:`Triggered`
    (`self.OnPlayerTernaryInteract`)))

(event `Dash`
  (bind _returnvalue (`self.K2_GetActorLocation`))
  (bind _returnvalue_2 (`PawnMovementComponent.GetLastInputVector` (`self.CharacterMovement`)))
  ; Dash
  (if (`self.IsDashLocked`)
    _
    (elif (not (`KismetMathLibrary.Vector_IsNearlyZero` _returnvalue_2))
      (`self.LockMovements`)
      (`self.Event LockAttack`)
      (`self.Event LockLookAtCursor`)
      (`self.LockDash`)
      (set `self.DashStartPos` _returnvalue)
      (set `self.DashEndPos` (+ _returnvalue (* _returnvalue_2 (`self.DashLenght`))))
      (`GameplayStatics.PlaySoundAtLocation` "/Game/Audio/Cue/SC_Dash.SC_Dash" _returnvalue (struct) 1.0 1.0 0.0 null null null null)
      (`self.PlayAnimMontage` "/Game/Gameplay/Player/Momiji/AM_Roll.AM_Roll")
      (bind (_direction _time) (`Timeline|Timeline` :!via `PlayFromStart`)
        (:`Update`
          (`self.K2_SetActorLocation` (`KismetMathLibrary.VLerp` (`self.DashStartPos`) (`self.DashEndPos`) _time) true)
          (`self.K2_SetActorRotation` (`KismetMathLibrary.Conv_VectorToRotator` (`KismetMathLibrary.Normal` (- (`self.DashEndPos`) (`self.DashStartPos`)))) true))
        (:`Finished`
          (`self.UnlockMovements`)
          (`self.Event UnlockAttack`)
          (`self.Event UnlockLookAtCursor`)
          (`KismetSystemLibrary.Delay` (`self.DashCooldown`))
          (`self.UnlockDash`))))))

(event `LockDash`
  ; Dash
  (set `self.IsDashLocked` true))

(event `UnlockDash`
  ; Dash
  (set `self.IsDashLocked` false))

(event `MovePhysicsHandleLocation`
  (params (TargetPosition :type "Vector Structure"))
  (`PhysicsHandleComponent.SetTargetLocation` (`self.PhysicsHandle`) TargetPosition))

(event `LockMovements`
  (bind _asbp_top_down_player_controller (cast `/Game/Gameplay/Player/BP_TopDownPlayerController` (`self.GetController`)))
  (`/Game/Gameplay/Player/BP_TopDownPlayerController.UnbindIMC` _asbp_top_down_player_controller))

(event `Event LockLookAtCursor`
  (bind _asbp_top_down_player_controller (cast `/Game/Gameplay/Player/BP_TopDownPlayerController` (`self.GetController`)))
  (set `TopDownPlayerController.bEnableMouseLook_TO_REVIEW` false _asbp_top_down_player_controller))

(event `UnlockMovements`
  (bind _asbp_top_down_player_controller (cast `/Game/Gameplay/Player/BP_TopDownPlayerController` (`self.GetController`)))
  (`/Game/Gameplay/Player/BP_TopDownPlayerController.BindIMC` _asbp_top_down_player_controller))

(event `SetSpeedByMultiplicator`
  (params (SpeedMultiplacator :type "Float (double-precision)"))
  (set `CharacterMovementComponent.MaxWalkSpeed` (* SpeedMultiplacator (`self.BaseMouSpeed`)) (`self.CharacterMovement`)))

(event `Event UnlockLookAtCursor`
  (bind _asbp_top_down_player_controller (cast `/Game/Gameplay/Player/BP_TopDownPlayerController` (`self.GetController`)))
  (set `TopDownPlayerController.bEnableMouseLook_TO_REVIEW` true _asbp_top_down_player_controller))

(event `self.HealthComponent.OnDeadEvent`
  (`self.Event LockLookAtCursor`)
  (`self.LockMovements`)
  (`self.Event LockAttack`)
  (`|PlayMontage` (`self.Mesh`) "/Game/Gameplay/Player/Momiji/AM_Death.AM_Death"
    (:`OnCompleted`
      (bind _asbp_top_down_player_controller (cast `/Game/Gameplay/Player/BP_TopDownPlayerController` (`self.GetController`)))
      (`/Game/Gameplay/Player/BP_TopDownPlayerController.Event OnPawnDead` _asbp_top_down_player_controller))))

(event `Event LockAttack`
  (set `self.IsAttackLocked` true))

(event `Event UnlockAttack`
  (set `self.IsAttackLocked` false))

(event `self.AttackInDirection`
  (params (Direction :type "Vector Structure (by ref)"))
  (if (not (`self.IsAttackLocked`))
    (`self.Event LockAttack`)
    (`self.LockDash`)
    (bind _returnvalue (`self.PlayAnimMontage` "/Game/Gameplay/Player/Momiji/AM_ThrowKunai.AM_ThrowKunai"))
    (`KismetSystemLibrary.Delay` _returnvalue)
    (`self.UnlockDash`)
    (`KismetSystemLibrary.Delay` (`self.AttackCooldown`))
    (`self.Event UnlockAttack`)))

(event `self.OnAttackStarted`
  (params (SkeletalMeshComponent :type "SkeletalMeshComponent Object Reference") (AnimSequenceBase :type "AnimSequenceBase Object Reference"))
  (bind _asweapon_base (cast `WeaponBase` (`self.MainItem`)))
  (bind _returnvalue (`WeaponBase.GetAttackOrigin` _asweapon_base))
  (`WeaponBase.AttackInDirection` _asweapon_base (`CombatActor.GetAttackDirection` _returnvalue))
  (`GameplayStatics.PlaySoundAtLocation` "/Game/Audio/Cue/SC_KunaiFire.SC_KunaiFire" _returnvalue (struct) 1.0 1.0 0.0 null null null null))

(event `Event OnPrayer`
  (`self.LockDash`)
  (`self.LockMovements`)
  (`self.Event LockLookAtCursor`)
  (bind _returnvalue (`self.PlayAnimMontage` "/Game/Gameplay/Player/Momiji/AM_Prayer.AM_Prayer"))
  (`KismetSystemLibrary.Delay` _returnvalue)
  (`self.UnlockDash`)
  (`self.Event UnlockAttack`)
  (`self.Event UnlockLookAtCursor`))

(event `/Game/Gameplay/BPI_FootstepSource.OnFootstep`
  (params (Foot :type "/Game/Gameplay/AI/Characters/Mannequins/Anims/Anims/E_Limb Enum" :default "NewEnumerator0") (Strength :type "Float (double-precision)") (MeshComp :type "SkeletalMeshComponent Object Reference") (Anim :type "AnimSequenceBase Object Reference"))
  (`AudioComponent.SetFloatParameter` (`self.StepEmitter`) "StepVolume" (`self.FootstepsVolume`))
  (`AudioComponent.Play` (`self.StepEmitter`) 0.0))

(fn `GetAttackMultiplier`
  (returns (ReturnValue :type "Float (single-precision)"))
  (return (`self.AttackDamageMultiplicator`)))

(fn `OnPrayerClap`
  (`GameplayStatics.PlaySoundAtLocation` "/Game/Audio/Cue/SC_HandsClap.SC_HandsClap" (`self.K2_GetActorLocation`) (struct) 0.7 1.0 0.0 null null null null))

(fn `OnRoomEntered`
  (set `self.IsInCombat` true))

(fn `OnRoomSolved`
  (set `self.IsInCombat` false))

(fn `UpdateCoinsCount`
  (params (CoinsIncrement :type Integer))
  (bind _output_get (set `self.CoinsCount` (+ CoinsIncrement (`self.CoinsCount`))))
  (`self.OnCoinsCountUpdated` _output_get))

(fn `UserConstructionScript`)