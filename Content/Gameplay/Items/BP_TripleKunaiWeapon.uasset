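; BP_TripleKunaiWeapon is a weapon Blueprint that, going by its name, throws three kunai in a spread.
; It overrides FireinDirection and calls the parent implementation three times in sequence, so the projectile logic stays in the parent class.
; The first shot follows the given direction, and the other two rotate it around the up vector by offsets derived from the Angle variable.
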(event `self.FireInDirection`
  (params (Direction :type "Vector Structure (by ref)"))
  (`|ExecutionSequence`
    (:`then_0`
      (`parent.FireInDirection` Direction))
    (:`then_1`
      (`parent.FireInDirection` (`KismetMathLibrary.RotateAngleAxis` Direction (`self.Angle`) (`KismetMathLibrary.Vector_Up`))))
    (:`then_2`
      (bind _result (`/Engine/EditorBlueprintResources/StandardMacros.NegateFloat` (`self.Angle`))
        (:`  `
          (`parent.FireInDirection` (`KismetMathLibrary.RotateAngleAxis` Direction _result (`KismetMathLibrary.Vector_Up`))))))))

(fn `UserConstructionScript`)