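; BP_KunaiLeftover is a short-lived kunai remnant actor that dissolves away and then removes itself.
; On BeginPlay it gives its static mesh a dynamic material instance, and the Decay timeline drives that material's DissolveAmount parameter.
; The actor destroys itself when the timeline finishes or when its owner is destroyed, whichever comes first.
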(event `self.ReceiveBeginPlay`
  (`|ExecutionSequence`
    (:`then_0`
      (bind _returnvalue (`KismetMaterialLibrary.CreateDynamicMaterialInstance` (`PrimitiveComponent.GetMaterial` (`self.StaticMesh`) 0)))
      (bind _output_get (set `self.DMI` _returnvalue))
      (`PrimitiveComponent.SetMaterial` (`self.StaticMesh`) 0 _output_get))
    (:`then_1`
      (add `self.OnDestroyed` (`self.GetOwner`) (delegate `Destroy`)))
    (:`then_2`
      (bind (_direction _opcaity) (`Timeline|Decay`)
        (:`Update`
          (`MaterialInstanceDynamic.SetScalarParameterValue` (`self.DMI`) "DissolveAmount" _opcaity))
        (:`Finished`
          (`self.K2_DestroyActor`))))))

(event `Destroy` :!signature `self.OnDestroyed`
  (params (DestroyedActor :type "Actor Object Reference"))
  (`self.K2_DestroyActor`))

(fn `UserConstructionScript`)