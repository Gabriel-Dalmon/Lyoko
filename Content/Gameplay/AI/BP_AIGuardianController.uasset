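; AI controller for a guardian character that runs a behavior tree and feeds it target, threat and state through the blackboard.
; AIPerception sets sensed player-tagged actors as the target and switches the state enum, changing state again when that target is lost without clearing it.
; Separate OnPerceived and OnForgotten events track the threatening actor and an IsPerceived flag, clearing both only when the current threat forgets.
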(event `self.ReceivePossess`
  (params (PossessedPawn :type "Pawn Object Reference"))
  ; On Possess
  ;;[0.2694 1 0.3817 0.5] Initialize Behavior Tree
  (bind _blackboardcomponent (`self.UseBlackboard` (`self.BlackboardAsset`)))
  (set `self.BlackboardComponent` _blackboardcomponent)
  (`self.RunBehaviorTree` (`self.BehaviorTreeAsset`)))

(event `self.AIPerception.OnTargetPerceptionUpdated`
  (params (Actor :type "Actor Object Reference") (Stimulus :type "AIStimulus Structure"))
  ; AIPerception Events
  (if Stimulus_bSuccessfullySensed
    ;; On Potential Target Perceived
    (if (`self.IsPotentialTarget` Actor)
      ;;;[0.8958 0.2286 0.3036 0.5] On Valid Target Perceived
      (`self.SetTargetActor` Actor)
      (`self.Set Behavior State` "NewEnumerator3"))
    (else
      ;; On Target Lost
      (if (`self.IsCurrentTarget` Actor)
        (`self.Set Behavior State` "NewEnumerator2")))))

(event `self.OnPerceived`
  (params (`Threat Actor` :type "Actor Object Reference"))
  ; Threaten Logic
  (`self.SetThreatActor` `Threat Actor`)
  (set `self.IsPerceived` true))

(event `self.OnForgotten`
  (params (`Threat Actor` :type "Actor Object Reference"))
  ; Threaten Logic
  (if (== `Threat Actor` (`self.GetCurrentThreatActor`))
    (`self.SetThreatActor` null)
    (set `self.IsPerceived` false)))

(fn `GetCurrentThreatActor`
  (returns (`Threat Actor` :type "Object Object Reference"))
  (return (`BlackboardComponent.GetValueAsObject` (`self.BlackboardComponent`) (`self.ThreatActorKey`))))

(fn `IsCurrentTarget`
  (params (Actor :type "Object Object Reference"))
  (returns (ReturnValue :type Boolean))
  (return (== Actor (`BlackboardComponent.GetValueAsObject` (`self.BlackboardComponent`) (`self.TargetActorKey`)))))

(fn `IsPotentialTarget`
  (params (Actor :type "Actor Object Reference"))
  (returns (ReturnValue :type Boolean))
  (return (`self.ActorHasTag` Actor (`self.PlayerTag`))))

(fn `Set Behavior State`
  (params (`New State` :type "/Game/Gameplay/AI/GuardianStates Enum" :default "NewEnumerator0"))
  (`BlackboardComponent.SetValueAsEnum` (`self.BlackboardComponent`) (`self.StateKey`) `New State`))

(fn `SetTargetActor`
  (params (`Target Actor` :type "Object Object Reference"))
  (`BlackboardComponent.SetValueAsObject` (`self.BlackboardComponent`) (`self.TargetActorKey`) `Target Actor`))

(fn `SetThreatActor`
  (params (ThreatActor :type "Object Object Reference"))
  (`BlackboardComponent.SetValueAsObject` (`self.BlackboardComponent`) (`self.ThreatActorKey`) ThreatActor))

(fn `UserConstructionScript`)