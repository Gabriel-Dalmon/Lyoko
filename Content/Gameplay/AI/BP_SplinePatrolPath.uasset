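; BP_SplinePatrolPath is an actor that defines an AI patrol path with a spline component.
; It wraps the spline in helper functions that return its length, the distance along it at a given location, and the location at a given distance, all in world space.
; It has no active event or construction logic, so it only serves as path data to query.
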(fn `Get Distance at Location along Path`
  (params (Location :type "Vector Structure (by ref)"))
  (returns (Distance :type "Float (double-precision)"))
  (return (`SplineComponent.GetDistanceAlongSplineAtLocation` (`self.Spline`) Location "World")))

(fn `Get Length`
  (returns (Length :type "Float (double-precision)"))
  (return (`SplineComponent.GetSplineLength` (`self.Spline`))))

(fn `Get Location at Distance along Path`
  (params (Distance :type "Float (double-precision)"))
  (returns (Location :type "Vector Structure"))
  (return (`SplineComponent.GetLocationAtDistanceAlongSpline` (`self.Spline`) Distance "World")))

(fn `UserConstructionScript`)